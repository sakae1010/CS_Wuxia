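; Player character Blueprint that adds a fading outline highlight to its mesh when highlighted.
; HighlightActor applies the dynamic material from GetOutlineMaterialInstance as the mesh overlay and drives its Alpha parameter with the FadeIn timeline.
; UnHighlightActor plays a second timeline in reverse on the same parameter, then clears the overlay when finished.
; BeginPlay, overlap, Tick and the construction script are empty.
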(event `HightlightInterface.HighlightActor`
  (bind _returnvalue (`self.GetOutlineMaterialInstance`))
  (`/Engine/EditorBlueprintResources/StandardMacros.IsValid` _returnvalue
    (:`Is Valid`
      (bind _output_get (set `self.OutlineMaterialDynamic` _returnvalue))
      (`MeshComponent.SetOverlayMaterial` (`self.Mesh`) _output_get)
      (`MaterialInstanceDynamic.SetScalarParameterValue` _output_get (`self.Alpha`) 1.0)
      (bind (_direction _alpha) (`Timeline|FadeIn` :!via `PlayFromStart`)
        (:`Update`
          (`MaterialInstanceDynamic.SetScalarParameterValue` (`self.OutlineMaterialDynamic`) (`self.Alpha`) _alpha))))))

(event `HightlightInterface.UnHighlightActor`
  (`/Engine/EditorBlueprintResources/StandardMacros.IsValid` (`self.OutlineMaterialDynamic`)
    (:`Is Valid`
      (`MaterialInstanceDynamic.SetScalarParameterValue` (`self.OutlineMaterialDynamic`) (`self.Alpha`) 1.0)
      (bind (_direction _alpha) (`Timeline|Timeline` :!via `ReverseFromEnd`)
        (:`Update`
          (`MaterialInstanceDynamic.SetScalarParameterValue` (`self.OutlineMaterialDynamic`) (`self.Alpha`) _alpha))
        (:`Finished`
          (`MeshComponent.SetOverlayMaterial` (`self.Mesh`) null))))))

(fn `UserConstructionScript`)